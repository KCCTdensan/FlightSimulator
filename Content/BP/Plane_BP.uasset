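; Plane Blueprint that flies at a constant step along world Y, with pitch driven by the Up input axis.
; Tick applies the offset, per frame without delta time, then sets absolute rotation, mapping pitch to X and roll to Y.
; Up input eases PitchValue with FInterpTo; roll and yaw are applied but never updated here.
; Tick also spins the propeller mesh by setting an incrementing world rotation.
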(event EventTick
  (params (DeltaSeconds :type Float%20%28single-precision%29))
  (Transformation|SetActorLocation (+ (Transformation|GetActorLocation) (Math|Vector|MakeVector 0.0 (Variables|Default|GetForward_Speed) 0.0)) false false)
  (Transformation|SetActorRotation (Math|Rotator|MakeRotator (Variables|Default|GetPitch_Value) (Variables|Default|GetRoll_Value) (Variables|Default|GetYaw_Value)))
  (Transformation|SetWorldRotation (Variables|Default|GetPlane_Propeller_Mesh) (Math|Rotator|MakeRotator 0.0 (Variables|Default|GetPropeller_Rotation) 0.0) false false)
  (Variables|Default|SetPropeller_Rotation (+ (Variables|Default|GetPropeller_Rotation) 5.0)))

(event Input|AxisEvents|InputAxisUp
  (params (AxisValue :type Float%20%28single-precision%29))
  (Variables|Default|SetPitch_Value (Math|Interpolation|FInterpTo (Variables|Default|GetPitch_Value) (* (Variables|Default|GetPitch_Speed) AxisValue) (Utilities|Time|GetWorldDeltaSeconds) 5.0)))

(fn ConstructionScript)