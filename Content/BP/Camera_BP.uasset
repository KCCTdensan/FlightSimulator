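; Camera actor that keeps itself aimed at the plane in the level.
; On BeginPlay it caches the first Plane_BP1 actor it finds.
; Each tick, while that plane is valid, it rotates the whole actor to look at the plane's location and resets the Camera component to zero relative location.
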(event EventTick
  (params (DeltaSeconds :type Float%20%28single-precision%29))
  (bind _plane (Variables|Default|GetPlane))
  (if (Utilities|IsValid _plane)
    (Transformation|SetActorRotation (Math|Rotator|FindLookatRotation (Transformation|GetActorLocation) (Transformation|GetActorLocation _plane)))
    (Transformation|SetRelativeLocation (Variables|Default|GetCamera) "0, 0,0.000000" false false)))

(event EventBeginPlay
  (bind _outactors (Actor|GetAllActorsOfClass "/Game/BP/Plane_BP1.Plane_BP1_C"))
  (Variables|Default|SetPlane (Utilities|Array|Get(acopy) _outactors)))

(fn ConstructionScript)